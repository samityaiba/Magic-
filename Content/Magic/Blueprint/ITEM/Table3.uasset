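; Table3 is an interactable item Blueprint that lets the player open and close a W_Table3 widget while near it.
; Overlapping its Box prints a prompt and enables input if player character 0 is a Test; ending overlap disables input.
; The C key drives a FlipFlop that creates or removes the widget and toggles the mouse cursor, though the prompt says E.
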(event OnComponentBeginOverlap(Box)
  (params (OverlappedComponent :type Primitive%20Component%20Object%20Reference) (OtherActor :type Actor%20Object%20Reference) (OtherComp :type Primitive%20Component%20Object%20Reference) (OtherBodyIndex :type Integer) (bFromSweep :type Boolean) (SweepResult :type Hit%20Result%20Structure%20%28by%20ref%29))
  (bind _astest (Utilities|Casting|CastToTest (Game|GetPlayerCharacter 0)))
  (bind _output_get (Variables|Default|SetPrintTime 6e+01))
  (Development|PrintString "Press Fucking E!" true true "(R=0.072053,G=1.000000,B=0.000000,A=1.000000)" _output_get)
  (Input|EnableInput (Game|GetPlayerController 0)))

(event OnComponentEndOverlap(Box)
  (params (OverlappedComponent :type Primitive%20Component%20Object%20Reference) (OtherActor :type Actor%20Object%20Reference) (OtherComp :type Primitive%20Component%20Object%20Reference) (OtherBodyIndex :type Integer))
  (Variables|Default|SetPrintTime 0.0)
  (Input|DisableInput (Game|GetPlayerController 0)))

(event Input|KeyboardEvents|C
  (params (Key :type Key%20Structure :default "None"))
  (bind _returnvalue (Game|GetPlayerController 0))
  (:Pressed
    (Utilities|FlowControl|FlipFlop
      (:A
        (Variables|/Script/Engine.PlayerController|SetbShowMouseCursor _returnvalue true)
        (bind _returnvalue_2 (UserInterface|CreateWidget "/Game/Magic/Blueprint/Widget/W_Table3.W_Table3_C"))
        (UserInterface|Viewport|AddtoViewport _returnvalue_2 0))
      (:B
        (Variables|/Script/Engine.PlayerController|SetbShowMouseCursor _returnvalue false)
        (Widget|RemovefromParent _returnvalue_2)))))

(fn ConstructionScript)