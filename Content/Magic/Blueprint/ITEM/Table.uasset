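; Table actor that spawns a product model on top of itself when the Test player character enters its box trigger.
; On overlap it shows a debug prompt to press E, though no input is handled here, and uses the player's WInfoRef table index to pick a product row name.
; The matching DT_Product row supplies the class to spawn, only while NewItem is invalid.
; BeginPlay caches an AIR actor as OldItem, unused here.
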(event OnComponentBeginOverlap(Box)
  (params (OverlappedComponent :type Primitive%20Component%20Object%20Reference) (OtherActor :type Actor%20Object%20Reference) (OtherComp :type Primitive%20Component%20Object%20Reference) (OtherBodyIndex :type Integer) (bFromSweep :type Boolean) (SweepResult :type Hit%20Result%20Structure%20%28by%20ref%29))
  (bind _astest (Utilities|Casting|CastToTest (Game|GetPlayerCharacter 0)))
  (bind _output_get (Variables|Default|SetPrintTime 6e+01))
  (Development|PrintString "Press Fucking E!" true true "(R=0.072053,G=1.000000,B=0.000000,A=1.000000)" _output_get)
  (bind _asgamemode_bp (Utilities|Casting|CastToGamemode_BP (Game|GetGameMode)))
  (bind _outrownames (DataTable|GetDataTableRowNames (Variables|/Game/Magic/Blueprint/Gamemode_BP.Gamemode_BP_C|Getproduct _asgamemode_bp)))
  (bind _returnvalue (Utilities|GetDataTableRow "/Game/Magic/Blueprint/DATA/DT_Product.DT_Product" (Utilities|Array|Get(acopy) _outrownames (Variables|/Game/Magic/Blueprint/Widget/W_Info.W_Info_C|GetindexForTable (Variables|/Game/Magic/Blueprint/Player/Test.Test_C|GetW_info_Ref _astest))))
    (:then
      (Variables|Default|GetNewItem
        (:then)
        (:else
          (bind _returnvalue_2 (Game|SpawnActorfromClass (.Model (Utilities|Struct|BreakS_product _returnvalue)) (Math|Conversions|ToTransform(Vector) (Math|Transform|TransformLocation (Transformation|GetActorTransform) "0.000000,0.000000,70.000000")) "Undefined" "MultiplyWithRoot" 0 0))
          (Variables|Default|SetNewItem _returnvalue_2))))))

(event OnComponentEndOverlap(Box)
  (params (OverlappedComponent :type Primitive%20Component%20Object%20Reference) (OtherActor :type Actor%20Object%20Reference) (OtherComp :type Primitive%20Component%20Object%20Reference) (OtherBodyIndex :type Integer))
  (Variables|Default|SetPrintTime 0.0))

(event EventBeginPlay
  (bind _returnvalue (Actor|GetActorOfClass "/Game/Magic/Blueprint/ITEM/AIR.AIR_C"))
  (Variables|Default|SetOldItem _returnvalue))

(event Input|KeyboardEvents|E
  (params (Key :type Key%20Structure)))

(fn ConstructionScript)