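; Game mode that tracks the day cycle of what appears to be a shop game, holding day, phase, time and play state.
; BeginPlay fetches a random product data table row without using it, then resets that state.
; End_Day advances the day, resets phase and timer, and fetches the player character and a Table3 actor.
; Income summing across three tables and the money update are disconnected, and playstart is empty.
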(event Custom|End_Day
  (Variables|Default|SetDay (+ (Variables|Default|GetDay) 1))
  (Variables|Default|SetPhease "NewEnumerator1")
  (Variables|Default|SetTime 0.0)
  (Variables|Default|SetIs%20play false)
  (bind _astest (Utilities|Casting|CastToTest (Game|GetPlayerCharacter 0)))
  (bind _returnvalue (Actor|GetActorOfClass "/Game/Magic/Blueprint/ITEM/Table3.Table3_C")))

(event Custom|play%20start)

(event EventTick
  (params (DeltaSeconds :type Float%20%28single-precision%29)))

(event EventBeginPlay
  (Utilities|FlowControl|Sequence
    (:then_0
      (bind _outrownames (DataTable|GetDataTableRowNames (Variables|Default|Getproduct)))
      (Utilities|GetDataTableRow "/Game/Magic/Blueprint/DATA/DT_Product.DT_Product" (.OutItem (Utilities|Array|Random _outrownames))))
    (:then_1
      (Variables|Default|SetDay 0)
      (Variables|Default|SetPhease "NewEnumerator1")
      (Variables|Default|SetTime 0.0)
      (Variables|Default|SetIs%20play false))))

(fn ConstructionScript)